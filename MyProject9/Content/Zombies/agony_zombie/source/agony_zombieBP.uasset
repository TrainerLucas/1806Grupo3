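; Zombie enemy character Blueprint that idles, chases the player and attacks, driven by a state enum through ActualizarEstad.
; Idle polls for a path and nearby player, AIMoveTo drives the chase into a timed attack animation, and failed moves return to idle.
; Hit reaction subtracts health, then applies physics knockback or ragdoll death.
; AnyDamage switches to idle, so nothing here triggers the hit or death states.
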(event `self.ReceiveBeginPlay`
  (`self.ActualizarEstad` "NewEnumerator0"))

(event `ActualizarEstad`
  (params (Enum :type "/Game/Zombies/agony_zombie/source/Enum_Agony Enum" :default "NewEnumerator0"))
  (bind _capsulecomponent (`self.CapsuleComponent`))
  (bind _output_get (set `self.EstadoDelZombie` Enum))
  (switch `/Game/Zombies/agony_zombie/source/Enum_Agony` _output_get
    (:`NewEnumerator0`
      (`SkeletalMeshComponent.PlayAnimation` (`self.Mesh`) "/Game/Zombies/agony_zombie/source/Zombie_Idle__3_.Zombie_Idle__3_" true)
      (bind _returnvalue (`NavigationSystemV1.FindPathToActorSynchronously` (`self.K2_GetActorLocation`) (`GameplayStatics.GetPlayerCharacter` 0) 50.0 null null :!label _label))
      (if (not (`NavigationPath.IsValid` _returnvalue))
        (`KismetSystemLibrary.Delay` 0.2 :!label _label_2)
        (goto _label)
        (elif (< (`KismetMathLibrary.VSizeXY` (- (`self.K2_GetActorLocation`) (`self.K2_GetActorLocation` (`GameplayStatics.GetPlayerCharacter` 0)))) 900.0)
          (`self.ActualizarEstad` "NewEnumerator1")
          (else
            (goto _label_2)))))
    (:`NewEnumerator1`
      (`SkeletalMeshComponent.PlayAnimation` (`self.Mesh`) "/Game/Zombies/agony_zombie/source/Zombie_Running__1_.Zombie_Running__1_" true)
      (`|AIMoveTo` self (0.0 0.0 0.0) (`GameplayStatics.GetPlayerCharacter` 0)
        (:`OnSuccess`
          (`self.ActualizarEstad` "NewEnumerator2"))
        (:`OnFail`
          (`self.ActualizarEstad` "NewEnumerator0"))))
    (:`NewEnumerator2`
      (`SkeletalMeshComponent.PlayAnimation` (`self.Mesh`) "/Game/Zombies/agony_zombie/source/Zombie_Attack__2_.Zombie_Attack__2_" true)
      (`KismetSystemLibrary.Delay` 2.36)
      (if (`|EnumInequality` (`self.EstadoDelZombie`) "NewEnumerator0")
        (`self.ActualizarEstad` "NewEnumerator1")))
    (:`NewEnumerator3`
      (`SkeletalMeshComponent.PlayAnimation` (`self.Mesh`) "/Game/Zombies/agony_zombie/source/Zombie_Reaction_Hit__2_.Zombie_Reaction_Hit__2_" false)
      (bind _output_get_2 (set `self.vida` (- (`self.vida`) (stale `self.ReceiveAnyDamage` Damage))))
      (if (<= _output_get_2 0.0)
        (`self.ActualizarEstad` "NewEnumerator4")
        (else
          (`PrimitiveComponent.SetSimulatePhysics` _capsulecomponent true)
          (`PrimitiveComponent.AddImpulse` _capsulecomponent (* (- (`self.K2_GetActorLocation`) (`self.K2_GetActorLocation` (`GameplayStatics.GetPlayerCharacter` 0)) (0.0 0.0 -10.0)) (100.0 100.0 100.0)) "None" false)
          (`KismetSystemLibrary.Delay` 2.0)
          (`PrimitiveComponent.SetSimulatePhysics` (`self.CapsuleComponent`) false)
          (`CharacterMovementComponent.SetMovementMode` (`self.CharacterMovement`) "MOVE_Walking" 0)
          (`self.ActualizarEstad` "NewEnumerator1"))))
    (:`NewEnumerator4`
      (`PrimitiveComponent.SetSimulatePhysics` (`self.Mesh`) true)
      (set `self.muerto` true))))

(event `self.ReceiveAnyDamage`
  (params (Damage :type "Float (single-precision)") (DamageType :type "DamageType Object Reference") (InstigatedBy :type "Controller Object Reference") (DamageCauser :type "Actor Object Reference"))
  (`self.ActualizarEstad` "NewEnumerator0"))

(fn `UserConstructionScript`)